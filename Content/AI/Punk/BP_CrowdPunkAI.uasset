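; AI controller for crowd punk enemies that spots hostile targets and alerts the rest of its group.
; It runs a behavior tree on BeginPlay and classifies perceived actors through a class-to-relation map, defaulting to Friendly.
; When it perceives an Enemy and has no valid Curr_Player, it writes that actor into the blackboard of every actor sharing its pawn's first tag, so the group targets together.
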(event OnTargetPerceptionUpdated(AIPerception)
  (params (Actor :type Actor%20Object%20Reference) (Stimulus :type AI%20Stimulus%20Structure))
  (switch Utilities|FlowControl|Switch|SwitchonE_Relationships (CallFunction|GetRelation Actor)
    (:NewEnumerator0
      (Utilities|IsValid (AI|Components|Blackboard|GetValueasObject (AI|GetBlackboard 0) (Utilities|Name|MakeLiteralName "Curr_Player"))
        (:Is%20Not%20Valid
          (bind _outactors (Actor|GetAllActorswithTag (Utilities|Array|Get(acopy) (Variables|/Script/Engine.Actor|GetTags (Pawn|GetControlledPawn)))))
          (for _array_element _outactors
            (if (Utilities|IsValid (AI|GetBlackboard _array_element))
              ;[1 1 1] KS: enemy (player) at the target of the attack
              (AI|Components|Blackboard|SetValueasObject (AI|GetBlackboard _array_element) (Utilities|Name|MakeLiteralName "Curr_Player") Actor)
              (Development|PrintString "got him!"))))))))

(event EventBeginPlay
  (AI|RunBehaviorTree (Variables|Default|GetBehaviorTree)))

(fn ConstructionScript)

(fn GetRelation
  (params (Target :type Actor%20Object%20Reference))
  (bind _returnvalue (Utilities|GetClass Target))
  (bind _relation (Variables|Default|GetRelation))
  (bind (_value _returnvalue_2) (Utilities|Map|Find _relation _returnvalue))
  (return (select _returnvalue_2 _value "NewEnumerator2")))