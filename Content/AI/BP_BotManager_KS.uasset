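; Manager actor for a crowd of AI bots that assigns a leader, formation slots and attack roles.
; On BeginPlay it makes the first bot leader, gives followers alternating sides with stepped distances, and copies its own tags to every bot.
; A looping timer reassigns front, left or right positions by array index, shown as overhead text.
; The self-destroy check for invalid bots is never scheduled.
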(event Custom|ManagingAttack
  ;[1 1 1] KS: *attackers
  (for (_array_element _array_index) (Variables|Default|GetBots)
    ;[1 1 1] KS: 0 index is leader
    (Variables|Default|SetCount _array_index)
    (if (not (== _array_index 0))
      ;[1 1 1] KS: only 1 to the "left"
      (if (== (Variables|Default|GetCount) 1)
        ;[1 1 1] KS: only 1 to the "right"
        (Utilities|IsValid _array_element
          (:Is%20Valid
            (Variables|/Game/AI/BP_AIBotBase_KS.BP_AIBotBase_KS_C|SetPosition _array_element 1)
            ;[1 1 1] KS: displays role overhead
            (Rendering|Components|TextRender|SetText (Variables|/Game/AI/BP_AIBotBase_KS.BP_AIBotBase_KS_C|GetTR_Crowd_role _array_element) (Utilities|Text|MakeLiteralText "front"))))
        (else
          ;[1 1 1] KS: crowd members 4+ go to the "right"
          (if (== (Variables|Default|GetCount) 2)
            (Utilities|IsValid _array_element
              (:Is%20Valid
                (Variables|/Game/AI/BP_AIBotBase_KS.BP_AIBotBase_KS_C|SetPosition _array_element 2)
                (Rendering|Components|TextRender|SetText (Variables|/Game/AI/BP_AIBotBase_KS.BP_AIBotBase_KS_C|GetTR_Crowd_role _array_element) (Utilities|Text|MakeLiteralText "left"))))
            (else
              (Utilities|IsValid _array_element
                (:Is%20Valid
                  (Variables|/Game/AI/BP_AIBotBase_KS.BP_AIBotBase_KS_C|SetPosition _array_element 3)
                  (Rendering|Components|TextRender|SetText (Variables|/Game/AI/BP_AIBotBase_KS.BP_AIBotBase_KS_C|GetTR_Crowd_role _array_element) (Utilities|Text|MakeLiteralText "right")))))))))))

(event Custom|CheckBots
  ;[1 1 1] for optimization
  (for _array_element (Variables|Default|GetBots)
    (if (not (Utilities|IsValid _array_element))
      (Actor|DestroyActor))))

(event EventBeginPlay
  (bind _bots (Variables|Default|GetBots))
  (Utilities|FlowControl|Sequence
    (:then_1
      ;[1 1 1] KS: sides assignment
      (for _index (range 1 (Utilities|Array|Length _bots))
        (Variables|Default|SetIndex_1+ _index)
        (Variables|Default|Setodd (== (Math|Integer|%(Integer) _index 2) 0))
        (Utilities|IsValid (Utilities|Array|Get(acopy) _bots _index)
          (:Is%20Valid
            (bind _output_get (Variables|Default|Setbot's_unit (Utilities|Array|Get(acopy) _bots _index)))
            ;[1 1 1] KS: sets 0 index as leader
            (bind _output_get_2 (Variables|/Game/AI/BP_AIBotBase_KS.BP_AIBotBase_KS_C|SetLeader _output_get (Utilities|Array|Get(acopy) _bots)))
            ;[1 1 1] KS: displays leader overhead
            (bind _asbp_aibot_base_ks (Utilities|Casting|CastToBP_AIBotBase_KS _output_get_2))
            (Rendering|Components|TextRender|SetText (Variables|/Game/AI/BP_AIBotBase_KS.BP_AIBotBase_KS_C|GetTR_Crowd_role _asbp_aibot_base_ks) (Utilities|Text|MakeLiteralText "leader"))
            (if (Variables|Default|Getodd)
              ;[1 1 1] KS: odd == side
              (Variables|/Game/AI/BP_AIBotBase_KS.BP_AIBotBase_KS_C|SetSide (Variables|Default|Getbot's_unit) (Variables|Default|Getodd))
              ;[1 1 1] KS: different distances for non leader
              (Variables|/Game/AI/BP_AIBotBase_KS.BP_AIBotBase_KS_C|SetDistance (Variables|Default|Getbot's_unit) (Math|Conversions|ToFloat(Integer) (* (- (Variables|Default|GetIndex_1+) 1) 100)))
              (else
                (Variables|/Game/AI/BP_AIBotBase_KS.BP_AIBotBase_KS_C|SetSide (Variables|Default|Getbot's_unit) (Variables|Default|Getodd))
                (Variables|/Game/AI/BP_AIBotBase_KS.BP_AIBotBase_KS_C|SetDistance (Variables|Default|Getbot's_unit) (Math|Conversions|ToFloat(Integer) (* (Variables|Default|GetIndex_1+) 100)))))))))
    (:then_2
      ;[1 1 1] KS: sets own tag to each bot
      (for _array_element (Variables|Default|GetBots)
        (if (Utilities|IsValid _array_element)
          (Variables|/Script/Engine.Actor|SetTags _array_element (Variables|Actor|GetTags)))))
    (:then_3
      ;[1 1 1] KS: Managing Attackers
      (Utilities|Time|SetTimerbyEvent (delegate Custom|ManagingAttack) 1.0 true))))

(fn ConstructionScript)